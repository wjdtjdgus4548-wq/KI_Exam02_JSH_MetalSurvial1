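; Flamethrower weapon Blueprint that burns BP_EnemyCharacter actors inside a damage box while firing.
; IA_Fire start and release drive a macro that toggles the Niagara flame, fades the looping audio and sets IsTurnOn, with debug prints.
; The first recorded enemy overlap starts a looping timer that damages all overlapping enemies while IsTurnOn is true.
; Any enemy leaving clears that timer, and OverlappedEnemies is never emptied.
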(event `EnhancedInput|/Game/Weapon/IA_Fire`
  (params (ActionValue :type Boolean) (ElapsedSeconds :type "Float (double-precision)") (TriggeredSeconds :type "Float (double-precision)") (InputAction :type "InputAction Object Reference" :default "/Game/Weapon/IA_Fire.IA_Fire"))
  (:`Started`
    (`self.화염방사기 메커니즘 완성(디버깅 해야됨)` :!label _label))
  (:`Completed`
    (goto _label :!via `execute2`)))

(event `self.DamegeBox.OnComponentBeginOverlap`
  (params (OverlappedComponent :type "PrimitiveComponent Object Reference") (OtherActor :type "Actor Object Reference") (OtherComp :type "PrimitiveComponent Object Reference") (OtherBodyIndex :type Integer) (bFromSweep :type Boolean) (SweepResult :type "HitResult Structure (by ref)"))
  (cast `/Game/Enemy2/BP_EnemyCharacter` OtherActor)
  (`KismetArrayLibrary.Array_AddUnique` (`self.OverlappedEnemies`))
  (if (== (`KismetArrayLibrary.Array_Length` (`self.OverlappedEnemies`)) 1)
    (bind _returnvalue (`KismetSystemLibrary.K2_SetTimerDelegate` (delegate `DealFireDamage`) 0.2 true))
    (set `self.DamegeTimmerHandle` _returnvalue)))

(event `DealFireDamage`
  (bind _overlappingactors (`PrimitiveComponent.GetOverlappingActors` (`self.DamegeBox`) "/Game/Enemy2/BP_EnemyCharacter.BP_EnemyCharacter_C"))
  (for _array_element _overlappingactors
    (if (`self.IsTurnOn?`)
      (`GameplayStatics.ApplyDamage` _array_element 5.0 null self)
      (else
        (`KismetSystemLibrary.PrintString` "데미지가 전달되지 않습니다.")))))

(event `self.DamegeBox.OnComponentEndOverlap`
  (params (OverlappedComponent :type "PrimitiveComponent Object Reference") (OtherActor :type "Actor Object Reference") (OtherComp :type "PrimitiveComponent Object Reference") (OtherBodyIndex :type Integer))
  (cast `/Game/Enemy2/BP_EnemyCharacter` OtherActor)
  (`KismetSystemLibrary.K2_ClearAndInvalidateTimerHandle` (`self.DamegeTimmerHandle`)))

(fn `StartFire()`
  (params (NewParam :type "/Game/Weapon/BP_Weapon_FlameThrower1 Object Reference")))

(fn `StopFire()`)

(fn `UserConstructionScript`)
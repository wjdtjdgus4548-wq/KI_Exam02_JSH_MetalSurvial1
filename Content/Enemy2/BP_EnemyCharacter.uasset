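; Enemy character that spots the player's OffroadCar_Pawn, plays a melee attack at close range, and dies when health runs out.
; AI perception writes a sensed car into the BP_EnemyController blackboard as TargetActor.
; Sphere overlap with the car plays a non-looping melee animation behind a timed IsAttacking lock, without applying damage itself.
; AnyDamage lowers health; at zero, Die stops movement, disables capsule collision and sets a short lifespan.
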(event `self.ReceiveAnyDamage`
  (params (Damage :type "Float (single-precision)") (DamageType :type "DamageType Object Reference") (InstigatedBy :type "Controller Object Reference") (DamageCauser :type "Actor Object Reference"))
  (`|ExecutionSequence`
    (:`then_0`
      (`KismetSystemLibrary.PrintString` "데미지 입는중")
      (bind _output_get (set `self.Current Health` (- (`self.Current Health`) Damage)))
      (`KismetSystemLibrary.PrintString` (`KismetStringLibrary.Conv_DoubleToString` _output_get))
      (set `self.bIsDead?` (<= (`self.Current Health`) 0.0))
      (`self.Die` false))))

(event `Die`
  (params (NewParam :type Boolean))
  (if (`self.bIsDead?`)
    (`MovementComponent.StopMovementImmediately` (`self.CharacterMovement`))
    (`CharacterMovementComponent.SetMovementMode` (`self.CharacterMovement`) "MOVE_None" 0)
    (`PrimitiveComponent.SetCollisionEnabled` (`self.CapsuleComponent`) "NoCollision")
    (`self.SetLifeSpan` 3.0)))

(event `self.AIPerception.OnTargetPerceptionUpdated`
  (params (Actor :type "Actor Object Reference") (Stimulus :type "AIStimulus Structure"))
  (if (`.bSuccessfullySensed` (break `AIStimulus` Stimulus))
    (bind `_as폰` (cast `Pawn` Actor))
    (bind _asoffroad_car_pawn (cast `/Game/ProjectPawn/Blueprints/OffroadCar/OffroadCar_Pawn` `_as폰`))
    (bind _returnvalue (`self.GetController`))
    (bind _asbp_enemy_controller (cast `/Game/Enemy2/BP_EnemyController` _returnvalue))
    (bind _returnvalue_2 (`AIBlueprintHelperLibrary.GetBlackboard` _asbp_enemy_controller))
    (`BlackboardComponent.SetValueAsObject` _returnvalue_2 (`self.Target Actor`) _asoffroad_car_pawn)))

(event `self.Sphere.OnComponentBeginOverlap`
  (params (OverlappedComponent :type "PrimitiveComponent Object Reference") (OtherActor :type "Actor Object Reference") (OtherComp :type "PrimitiveComponent Object Reference") (OtherBodyIndex :type Integer) (bFromSweep :type Boolean) (SweepResult :type "HitResult Structure (by ref)"))
  (cast `/Game/ProjectPawn/Blueprints/OffroadCar/OffroadCar_Pawn` OtherActor)
  (if (not (`self.IsAttacking`))
    (set `self.IsAttacking` true)
    (set `CharacterMovementComponent.MaxWalkSpeed` (`self.DefaultWalkSpedd`) (`self.CharacterMovement`))
    (bind _returnvalue (`self.GetController`))
    (cast `/Game/Enemy2/BP_EnemyController` _returnvalue)
    (`SkeletalMeshComponent.Stop` (`self.Mesh`))
    (`SkeletalMeshComponent.PlayAnimation` (`self.Mesh`) "/Game/Enemy2/AM_Enemy_Melee.AM_Enemy_Melee" false)
    (`KismetSystemLibrary.Delay` 5.0)
    (set `CharacterMovementComponent.MaxWalkSpeed` (`self.DefaultWalkSpedd`) (`self.CharacterMovement`))
    (set `self.IsAttacking` false)))

(event `self.ReceiveBeginPlay`
  (set `self.DefaultWalkSpedd` (`CharacterMovementComponent.MaxWalkSpeed` (`self.CharacterMovement`))))

(fn `UserConstructionScript`)
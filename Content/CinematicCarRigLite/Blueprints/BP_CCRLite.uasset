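; Lite cinematic car rig actor that assembles a car from body, wheel and caliper meshes and spins its wheels as it moves.
; Construction creates and places the parts using axle offsets and mesh bounds.
; Each update optionally ground-snaps via a line trace with interpolated slope alignment, resets the pose, then derives wheel spin, including extra wheels, from accumulated body travel.
; A looping EditorTick timer started in construction repeats Tick's update chain.
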(event `self.ReceiveTick`
  (params (DeltaSeconds :type "Float (single-precision)"))
  (set `self.DeltaSeconds` DeltaSeconds)
  (`self.Actor Ground Snap` :!label _label)
  (`self.Initial State`)
  (`self.Wheel Drive`))

(event `/Game/CinematicCarRigLite/Blueprints/BI_CCRLiteEditorTick.EditorTick`
  (goto _label))

(fn `Actor Ground Snap`
  (bind (_returnvalue_roll _returnvalue_pitch _returnvalue_yaw) (`KismetMathLibrary.BreakRotator` (`self.K2_GetActorRotation`)))
  (bind (_start_location _end_location) (`self.Trace Start End` (`self.K2_GetActorLocation`) (`self.GetActorUpVector`) (`.Z` (`self.Mesh Dimensions` (`self.BodyMesh`)))))
  (if (`self.StickToTheGround`)
    (bind _outhit (`KismetSystemLibrary.LineTraceSingle` :`Start` _start_location :`End` _end_location :`TraceChannel` "TraceTypeQuery1" :`bTraceComplex` true :`TraceColor` (struct :`R` 1.0 :`G` 1.0 :`A` 1.0) :`DrawTime` 0.05))
    (if (`GameplayStatics.BreakHitResult` _outhit)
      (`self.K2_SetActorLocationAndRotation` (`KismetMathLibrary.VInterpTo` (`self.K2_GetActorLocation`) (`.ImpactPoint` (`GameplayStatics.BreakHitResult` _outhit)) (`self.DeltaSeconds`)) (`KismetMathLibrary.MakeRotator` 0.0 0.0 _returnvalue_yaw))
      (set `self.ChassisRotation` (`KismetMathLibrary.RInterpTo` (`self.ChassisRotation`) (`KismetMathLibrary.MakeRotFromZX` (`.Normal` (`GameplayStatics.BreakHitResult` _outhit)) (`self.GetActorForwardVector`)) (`self.DeltaSeconds`) 5.0)))
    (else
      (set `self.ChassisRotation` (`self.K2_GetActorRotation`)))))

(fn `Components Creation`
  (`StaticMeshComponent.SetStaticMesh` (`self.Body`) (`self.BodyMesh`))
  (set `self.ExtraWheels` (`SceneComponent.GetChildrenComponents` (`self.Extra Wheels`) false))
  (`|ExecutionSequence`
    (:`then_0`
      (for _index (range 4)
        (bind _returnvalue (`AddComponent|NODE_AddStaticMeshComponent-17` :`bManualAttachment` true))
        (`StaticMeshComponent.SetStaticMesh` _returnvalue (select `bool` (> _index 1) :`false` (`self.FrontWheelMesh`) :`true` (`self.RearWheelMesh`)))
        (`SceneComponent.K2_AttachToComponent` _returnvalue (`self.Chassis`) "None" "KeepRelative" "KeepRelative" "KeepRelative" true)
        (`BlueprintMapLibrary.Map_Add` (`self.WheelsMap`) (`|GetArrayItem` (`self.SocketNames`) _index) _returnvalue)))
    (:`then_1`
      (for _index_2 (range 4)
        (bind _returnvalue_2 (`AddComponent|NODE_AddStaticMeshComponent-18` :`bManualAttachment` true))
        (`StaticMeshComponent.SetStaticMesh` _returnvalue_2 (select `bool` (> _index_2 1) :`false` (`self.FrontCaliperMesh`) :`true` (`self.RearCaliperMesh`)))
        (`SceneComponent.K2_AttachToComponent` _returnvalue_2 (`self.Chassis`) "None" "KeepRelative" "KeepRelative" "KeepRelative" true)
        (`BlueprintMapLibrary.Map_Add` (`self.CalipersMap`) (`|GetArrayItem` (`self.SocketNames`) _index_2) _returnvalue_2)))))

(fn `Initial State`
  (bind _chassis (`self.Chassis`))
  (bind (_x _y _z) (`self.Mesh Dimensions` (`self.RearWheelMesh`)))
  (bind (_x_2 _y_2 _z_2) (`self.Mesh Dimensions` (`self.FrontWheelMesh`)))
  (`self.SetActorScale3D` (1.0 1.0 1.0))
  (`SceneComponent.K2_SetWorldRotation` _chassis (`self.ChassisRotation`) false false)
  (`SceneComponent.K2_SetWorldLocation` _chassis (+ (`self.K2_GetActorLocation`) (* (`SceneComponent.GetUpVector` (`self.Chassis`)) (/ (+ _z_2 _z) 4.0))) false false)
  (`SceneComponent.SetWorldScale3D` _chassis (1.0 1.0 1.0))
  (`SceneComponent.K2_SetRelativeTransform` (`self.Body`) (`KismetMathLibrary.MakeTransform` (`KismetMathLibrary.MakeVector` 0.0 0.0 (`self.BodyHeight`))) false false)
  (`|ExecutionSequence`
    (:`then_0`
      (for _array_element (`self.SocketNames`)
        (bind _returnvalue (`KismetStringLibrary.Contains` _array_element "Front"))
        (bind _returnvalue_2 (`KismetMathLibrary.SelectFloat` (`self.FrontOffset`) (* (`self.RearOffset`) -1.0) _returnvalue))
        (bind _returnvalue_3 (`KismetStringLibrary.Contains` _array_element "Right"))
        (bind _returnvalue_4 (* (`KismetMathLibrary.SelectFloat` (`self.FrontSideOffset`) (`self.RearSideOffset`) _returnvalue) (`KismetMathLibrary.SelectFloat` 1.0 -1.0 _returnvalue_3)))
        (bind _returnvalue_5 (`KismetMathLibrary.SelectFloat` (/ (- _z_2 _z) 4.0) (/ (- _z _z_2) 4.0) _returnvalue))
        (`SceneComponent.K2_SetRelativeTransform` (`BlueprintMapLibrary.Map_Find` (`self.WheelsMap`) _array_element) (`KismetMathLibrary.MakeTransform` (`KismetMathLibrary.MakeVector` _returnvalue_2 _returnvalue_4 _returnvalue_5) (`KismetMathLibrary.MakeRotator` 0.0 0.0 (`KismetMathLibrary.SelectFloat` 0.0 180.0 _returnvalue_3))) false false)
        (`SceneComponent.K2_SetRelativeTransform` (`BlueprintMapLibrary.Map_Find` (`self.CalipersMap`) _array_element) (`KismetMathLibrary.MakeTransform` (`KismetMathLibrary.MakeVector` _returnvalue_2 _returnvalue_4 _returnvalue_5) (struct) (`KismetMathLibrary.MakeVector` 1.0 (`KismetMathLibrary.SelectFloat` 1.0 -1.0 _returnvalue_3) 1.0)) false false)))
    (:`then_1`
      (if (> (`KismetArrayLibrary.Array_Length` (`self.ExtraWheels`)) 0)
        (for _array_element_2 (`self.ExtraWheels`)
          (`SceneComponent.K2_SetRelativeRotation` :`self` _array_element_2))))))

(fn `StartEditorTick`
  (`KismetSystemLibrary.K2_SetTimer` null "EditorTick" 0.04 true)
  (set `self.DeltaSeconds` 0.04))

(fn `UserConstructionScript`
  (`self.StartEditorTick`)
  (`self.Components Creation`)
  (`self.Actor Ground Snap`)
  (`self.Initial State`)
  (`self.Wheel Drive`))

(fn `Wheel Drive`
  (bind (_distance_step _new_last_location) (`self.Body Distance Step` (`self.Body`) (`self.Last Location`)))
  (set `self.DistanceStep` _distance_step)
  (set `self.Last Location` _new_last_location)
  (bind _wheel_rotation_output (`self.Wheel Rotation` (`self.DistanceStep`) (`self.WheelRotation`)))
  (set `self.WheelRotation` _wheel_rotation_output)
  (for _array_element (`self.SocketNames`)
    (`SceneComponent.K2_AddLocalRotation` (`BlueprintMapLibrary.Map_Find` (`self.WheelsMap`) _array_element) (`KismetMathLibrary.MakeRotator` 0.0 (* (/ (`self.WheelRotation`) (* 3.14 (`KismetMathLibrary.SelectFloat` (`.Z` (`self.Mesh Dimensions` (`self.FrontWheelMesh`))) (`.Z` (`self.Mesh Dimensions` (`self.RearWheelMesh`))) (`KismetStringLibrary.Contains` _array_element "Front")))) (`KismetMathLibrary.SelectFloat` -1.0 1.0 (`KismetStringLibrary.Contains` _array_element "Right")))) false false))
  (for _array_element_2 (`self.ExtraWheels`)
    (`SceneComponent.K2_AddLocalRotation` _array_element_2 (`KismetMathLibrary.MakeRotator` 0.0 (/ (`self.WheelRotation`) (* 3.14 (`.SphereRadius` (`KismetSystemLibrary.GetComponentBounds` _array_element_2)) -2.0))) false false)))

(fn `Wheel Rotation`
  (params (`Distance Step` :type "Float (double-precision)") (`Wheel Rotation` :type "Float (double-precision)"))
  (returns (`Wheel Rotation Output` :type "Float (double-precision)"))
  (locals (WheelRotationLV :type "Float (double-precision)") (WheelRotationStepLV :type "Float (double-precision)"))
  (return (`KismetMathLibrary.SelectFloat` `Wheel Rotation` (+ `Wheel Rotation` (* `Distance Step` 360.0)) (== `Distance Step` 0.0))))
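; BP_MovingBox is a demo-level actor for Cinematic Car Rig Lite that slides back and forth along the world Y axis.
; Each tick offsets it from InitialTransform by a sine of game time scaled by Distance and Speed, keeping the initial rotation.
; The construction script starts a looping 60 Hz timer calling EditorTick, which reuses the Tick logic for in-editor animation.
; A Perlin noise graph is present but unused.
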(event `self.ReceiveTick`
  (params (DeltaSeconds :type "Float (single-precision)"))
  (bind (_initialtransform_location _initialtransform_rotation) (`KismetMathLibrary.BreakTransform` (`self.InitialTransform`)))
  (`self.K2_SetActorTransform` (`KismetMathLibrary.MakeTransform` (+ (`KismetMathLibrary.MakeVector` 0.0 (* (`self.Distance`) (`KismetMathLibrary.DegSin` (* (`KismetSystemLibrary.GetGameTimeInSeconds`) (* 75.0 (`self.Speed`)))))) _initialtransform_location) _initialtransform_rotation) :!label _label))

(event `/Game/CinematicCarRigLite/Blueprints/BI_CCRLiteEditorTick.EditorTick`
  (goto _label))

(fn `UserConstructionScript`
  (`KismetSystemLibrary.K2_SetTimer` null "EditorTick" 0.016667 true))